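; MainPlayerCharacter is the player character Blueprint, adding a main attack that works with the game's time-rewind system.
; Attack input, ignored while the RewindManager is manipulating time, plays a rewindable montage on the mesh using base, backward and slow variants.
; A DoOnce gate blocks repeat attacks until the montage completion event returns the "MainAttack" callback name and resets it.
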(event `self.ReceiveBeginPlay`
  (`parent.ReceiveBeginPlay`))

(event `InputAction|MainAttack`
  (params (Key :type "Key Structure"))
  (:`Pressed`
    (if (not (`/Game/Blueprints/RewindManager/RewindManager.IsTimeManipulationInProgress` (`self.RewindManager`)))
      (`/Engine/EditorBlueprintResources/StandardMacros.DoOnce` false :!label _label
        (:`Completed`
          (`self.PlayRewindableMontage` (`self.Mesh`) "/Game/Animations/Character/Attack/AttackBaseMontage.AttackBaseMontage" "/Game/Animations/Character/Attack/AttackBackwardMontage.AttackBackwardMontage" "/Game/Animations/Character/Attack/AttackSlowMontage.AttackSlowMontage" 1.0 0.0 "None" "MainAttack"))))))

(event `self.OnCompleteRewindableMontage`
  (params (Name :type "Name (by ref)"))
  (if (== Name "MainAttack")
    (goto _label :!via `Reset`)))

(fn `UserConstructionScript`)