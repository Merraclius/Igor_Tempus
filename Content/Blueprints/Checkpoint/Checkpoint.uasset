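; Checkpoint actor that registers itself as the active checkpoint when something overlaps its Cube.
; It finds the CheckpointSystem component on the game mode at BeginPlay and notifies it on every overlap, without filtering the overlapping actor.
; An inactive checkpoint then activates, swapping the cube's glass material and playing a brief Niagara burst.
; A Deactivate event restores the blue glass and clears the active flag, but nothing here calls it.
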(event `self.ReceiveBeginPlay`
  (set `self.CheckpointSystem` (`self.GetComponentByClass` (`GameplayStatics.GetGameMode`) "/Game/Blueprints/Checkpoint/CheckpointSystem.CheckpointSystem_C")))

(event `self.Cube.OnComponentBeginOverlap`
  (params (OverlappedComponent :type "PrimitiveComponent Object Reference") (OtherActor :type "Actor Object Reference") (OtherComp :type "PrimitiveComponent Object Reference") (OtherBodyIndex :type Integer) (bFromSweep :type Boolean) (SweepResult :type "HitResult Structure (by ref)"))
  (`/Game/Blueprints/Checkpoint/CheckpointSystem.RegisterActiveCheckpoint` (`self.CheckpointSystem`) self)
  (if (not (`self.IsActive`))
    (`self.Activate`)))

(event `Activate`
  (set `self.IsActive` true)
  (`PrimitiveComponent.SetMaterial` (`self.Cube`) 0 "/Game/Materials/BlueWhiteGlass.BlueWhiteGlass")
  (`ActorComponent.Activate` (`self.Niagara`) false)
  (`KismetSystemLibrary.Delay` 1.0)
  (`ActorComponent.Deactivate` (`self.Niagara`)))

(event `Deactivate`
  (set `self.IsActive` false)
  (`PrimitiveComponent.SetMaterial` (`self.Cube`) 0 "/Game/Materials/BlueGlass.BlueGlass"))

(fn `UserConstructionScript`)