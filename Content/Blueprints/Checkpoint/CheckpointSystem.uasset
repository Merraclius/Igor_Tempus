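; Checkpoint manager that tracks which single checkpoint is currently active in the game.
; Registering a new checkpoint deactivates the previous one, if it is valid and different, then stores the new reference.
; Queries report whether a given checkpoint is active and return the world location and rotation of the active checkpoint's Cube component, or zeros when none is valid.
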(fn `GetActiveCheckpointParams`
  (returns (Location :type "Vector Structure") (Rotation :type "Rotator Structure"))
  (bind _activecheckpoint (`self.ActiveCheckpoint`))
  (bind _cube (`/Game/Blueprints/Checkpoint/Checkpoint.Cube` _activecheckpoint))
  (if (`KismetSystemLibrary.IsValid` _activecheckpoint)
    (return (`SceneComponent.K2_GetComponentLocation` _cube) (`SceneComponent.K2_GetComponentRotation` _cube))
    (else
      (return (0.0 0.0 0.0)))))

(fn `IsActiveCheckpoint`
  (params (Checlpoint :type "/Game/Blueprints/Checkpoint/Checkpoint Object Reference"))
  (returns (IsActive :type Boolean))
  (return (== Checlpoint (`self.ActiveCheckpoint`))))

(fn `RegisterActiveCheckpoint`
  (params (Checkpoint :type "/Game/Blueprints/Checkpoint/Checkpoint Object Reference"))
  (bind _activecheckpoint (`self.ActiveCheckpoint`))
  (if (`KismetSystemLibrary.IsValid` _activecheckpoint)
    (if (not (== _activecheckpoint Checkpoint))
      (`/Game/Blueprints/Checkpoint/Checkpoint.Deactivate` _activecheckpoint)
      (set `self.ActiveCheckpoint` Checkpoint :!label _label))
    (else
      (goto _label))))