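; Base actor for rewindable objects, which records and restores the world transform of a designated component by state index.
; It caches the GameMode's RewindManager and stores states in a map, with events to collect, apply and remove them.
; Applying a missing index lerps between the surrounding multiples of 100, allowing sparse keyframes.
; Empty StartCollect and StartApply events run before each collect or apply, serving as hooks.
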(event `self.ReceiveBeginPlay`
  (set `self.RewindManager` (`self.GetComponentByClass` (`GameplayStatics.GetGameMode`) "/Game/Blueprints/RewindManager/RewindManager.RewindManager_C")))

(event `/Game/Blueprints/RewindManager/Rewindable.ApplyRewindState`
  (params (StateIndex :type Integer) (IsBackward :type Boolean))
  (bind _rewindablecomponent (`self.RewindableComponent`))
  (bind _rewindstates (`self.RewindStates`))
  (bind (_value _returnvalue) (`BlueprintMapLibrary.Map_Find` (`self.RewindStates`) StateIndex))
  (bind _returnvalue_2 (* (/ StateIndex 100) 100))
  (`self.StartApplyRewindState`)
  (if _returnvalue
    (`SceneComponent.K2_SetWorldTransform` _rewindablecomponent (`.Transform_2_6075E1B84316F2D437DB0A86274AD0AB` (break `/Game/Blueprints/RewindManager/RewindState` _value)) false false)
    (else
      (`SceneComponent.K2_SetWorldTransform` _rewindablecomponent (`KismetMathLibrary.TLerp` (`.Transform_2_6075E1B84316F2D437DB0A86274AD0AB` (break `/Game/Blueprints/RewindManager/RewindState` (`BlueprintMapLibrary.Map_Find` _rewindstates _returnvalue_2))) (`.Transform_2_6075E1B84316F2D437DB0A86274AD0AB` (break `/Game/Blueprints/RewindManager/RewindState` (`BlueprintMapLibrary.Map_Find` _rewindstates (+ _returnvalue_2 100)))) (* (`KismetMathLibrary.Conv_IntToDouble` (mod StateIndex 100)) 0.01)) false false))))

(event `/Game/Blueprints/RewindManager/Rewindable.CollectRewindState`
  (params (StateIndex :type Integer))
  (`self.StartCollectRewindState`)
  (`BlueprintMapLibrary.Map_Add` (`self.RewindStates`) StateIndex (make `/Game/Blueprints/RewindManager/RewindState` (`SceneComponent.K2_GetComponentToWorld` (`self.RewindableComponent`)))))

(event `/Game/Blueprints/RewindManager/Rewindable.RemoveRewindState`
  (params (StateIndex :type Integer))
  (`BlueprintMapLibrary.Map_Remove` (`self.RewindStates`) StateIndex))

(event `StartCollectRewindState`)

(event `StartApplyRewindState`)

(event `/Game/Blueprints/RewindManager/Rewindable.SetRewindableComponent`
  (params (Component :type "SceneComponent Object Reference"))
  (set `self.RewindableComponent` Component))

(fn `UserConstructionScript`)