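; Base character for the time-rewind system, recording indexed state snapshots and replaying them during time manipulation.
; SetRewindable and PlayRewindableMontage events buffer changes, which CollectRewindState stores in a map with the transform.
; ApplyRewindState restores snapshots, choosing old or new material and collision by direction, and lerps transforms between 100-step indices for missing states.
; Montages rewind through paired backward assets with mirrored start positions, and StopRepeat can resume the interrupted montage.
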(event `/Game/Blueprints/RewindManager/Rewindable.ApplyRewindState`
  (params (StateIndex :type Integer) (IsBackward :type Boolean))
  (bind _rewindablecomponent (`self.RewindableComponent`))
  (bind _rewindstates (`self.RewindStates`))
  (bind ((`Transform_2_6075E1B84316F2D437DB0A86274AD0AB` _transform) (`IsDeath_36_C4590F20474FC979CE75EB84DFC1FD49` _isdeath)) (break `/Game/Blueprints/RewindManager/RewindState` (`self.ActiveRewindState`)))
  (bind (_transform_2 _montagestate) (break `/Game/Blueprints/RewindManager/RewindState` (`self.ActiveRewindState`)))
  (bind (_transform_3 _montagestate_2) (break `/Game/Blueprints/RewindManager/RewindState` (`self.ActiveRewindState`)))
  (bind (_transform_4 _montagestate_3) (break `/Game/Blueprints/RewindManager/RewindState` (`self.ActiveRewindState`)))
  (bind ((`MaterialState_39_7E7AF8CB4B7103A9E1846FABC434A633` _materialstate) (`CollisionResponseToChannelState_42_62FF876241AADB85D775BB80273F9EDA` _collisionresponsetochannelstate) (`Integers_34_D45383FA4A24616AFCBAE89E259B4056` _integers)) (break `/Game/Blueprints/RewindManager/RewindState` (`self.ActiveRewindState`)))
  (bind (_value _returnvalue) (`BlueprintMapLibrary.Map_Find` (`self.RewindStates`) StateIndex))
  (bind _returnvalue_2 (* (/ StateIndex 100) 100))
  (bind (_materialtarget _index _newmaterial _oldmaterial) (break `/Game/Blueprints/RewindManager/RewindMaterialState` (`.MaterialState_39_7E7AF8CB4B7103A9E1846FABC434A633` (break `/Game/Blueprints/RewindManager/RewindState` (`self.ActiveRewindState`)))))
  (bind (_target _channel _newresponse _oldresponse) (break `/Game/Blueprints/RewindManager/RewindCollisionResponseToChannelState` (`.CollisionResponseToChannelState_42_62FF876241AADB85D775BB80273F9EDA` (break `/Game/Blueprints/RewindManager/RewindState` (`self.ActiveRewindState`)))))
  (bind _returnvalue_3 (`KismetSystemLibrary.IsValid` (`.ActiveMontage_22_4F3423F642A15DF5B8F1FDBC68FC0E34` (break `/Game/Blueprints/RewindManager/RewindMontageState` _montagestate))))
  (bind _returnvalue_4 (`SkeletalMeshComponent.GetAnimInstance` (break `/Game/Blueprints/RewindManager/RewindMontageState` _montagestate)))
  (if (`self.IsRewindEnabled`)
    (set `self.ActiveStateIsBackward` IsBackward)
    (set `self.ActiveRewindState` _value)
    (if _returnvalue
      (`SceneComponent.K2_SetWorldTransform` _rewindablecomponent _transform false false)
      (`self.ApplyRewindableIsDeath` _isdeath)
      (if (`KismetSystemLibrary.IsValid` _target)
        (if (`self.ActiveStateIsBackward`)
          (`PrimitiveComponent.SetCollisionResponseToChannel` _target _channel _oldresponse)
          (else
            (`PrimitiveComponent.SetCollisionResponseToChannel` _target _channel _newresponse))))
      (if (`KismetSystemLibrary.IsValid` _materialtarget)
        (if (`self.ActiveStateIsBackward`)
          (`PrimitiveComponent.SetMaterial` _materialtarget _index _oldmaterial)
          (else
            (`PrimitiveComponent.SetMaterial` _materialtarget _index _newmaterial))))
      (bind _keys (`BlueprintMapLibrary.Map_Keys` _integers))
      (for _array_element _keys
        (`self.ApplyRewindalbeInteger` _array_element (`BlueprintMapLibrary.Map_Find` _integers _array_element)))
      (if (and (`KismetSystemLibrary.IsValid` (`.BackwardMontage_15_52C2169F4294B3CFA2B3D5B1071283FE` (break `/Game/Blueprints/RewindManager/RewindMontageState` _montagestate_2))) (`self.ActiveStateIsBackward`))
        (set `self.IsActiveMontageHandled` true)
        (`|PlayMontage` (break `/Game/Blueprints/RewindManager/RewindMontageState` _montagestate_2) (`.BackwardMontage_15_52C2169F4294B3CFA2B3D5B1071283FE` (break `/Game/Blueprints/RewindManager/RewindMontageState` _montagestate_2)) 1.0 (`.BackwardStartPosition_27_2B9660444AFEEAA2F9C65FB0F6E36A75` (break `/Game/Blueprints/RewindManager/RewindMontageState` _montagestate_2)))
        (else
          (if _returnvalue_3
            (set `self.RewindableActiveMontage` (`.ActiveMontage_22_4F3423F642A15DF5B8F1FDBC68FC0E34` (break `/Game/Blueprints/RewindManager/RewindMontageState` _montagestate))))
          (if (and _returnvalue_3 (not (`self.IsActiveMontageHandled`)))
            (set `self.IsActiveMontageHandled` true)
            (set `self.ActiveMontagePositionLastPosition` (`AnimInstance.Montage_GetPosition` _returnvalue_4 (`.ActiveMontage_22_4F3423F642A15DF5B8F1FDBC68FC0E34` (break `/Game/Blueprints/RewindManager/RewindMontageState` _montagestate))))
            (`AnimInstance.Montage_Stop` _returnvalue_4 0.0 (`.ActiveMontage_22_4F3423F642A15DF5B8F1FDBC68FC0E34` (break `/Game/Blueprints/RewindManager/RewindMontageState` _montagestate)))
            (if (`KismetSystemLibrary.IsValid` (`.ActiveBackwardMontage_24_0B3D55604867C468FE8E56BE4CEE7420` (break `/Game/Blueprints/RewindManager/RewindMontageState` _montagestate)))
              (`|PlayMontage` (break `/Game/Blueprints/RewindManager/RewindMontageState` _montagestate) (`.ActiveBackwardMontage_24_0B3D55604867C468FE8E56BE4CEE7420` (break `/Game/Blueprints/RewindManager/RewindMontageState` _montagestate)) 1.0 (- (`AnimSequenceBase.SequenceLength` (`.ActiveBackwardMontage_24_0B3D55604867C468FE8E56BE4CEE7420` (break `/Game/Blueprints/RewindManager/RewindMontageState` _montagestate))) (`self.ActiveMontagePositionLastPosition`))
                (:`then`
                  _))))
          (if (and (`KismetSystemLibrary.IsValid` (`.SlowMontage_16_036E95F24CB735F24B141BB290ABAEF3` (break `/Game/Blueprints/RewindManager/RewindMontageState` _montagestate_3))) (not (`self.ActiveStateIsBackward`)))
            (`|PlayMontage` (break `/Game/Blueprints/RewindManager/RewindMontageState` _montagestate_3) (`.SlowMontage_16_036E95F24CB735F24B141BB290ABAEF3` (break `/Game/Blueprints/RewindManager/RewindMontageState` _montagestate_3))))))
      (else
        (`SceneComponent.K2_SetWorldTransform` _rewindablecomponent (`KismetMathLibrary.TLerp` (`.Transform_2_6075E1B84316F2D437DB0A86274AD0AB` (break `/Game/Blueprints/RewindManager/RewindState` (`BlueprintMapLibrary.Map_Find` _rewindstates _returnvalue_2))) (`.Transform_2_6075E1B84316F2D437DB0A86274AD0AB` (break `/Game/Blueprints/RewindManager/RewindState` (`BlueprintMapLibrary.Map_Find` _rewindstates (+ _returnvalue_2 100)))) (* (`KismetMathLibrary.Conv_IntToDouble` (mod StateIndex 100)) 0.01)) false false)))))

(event `/Game/Blueprints/RewindManager/Rewindable.CollectRewindState`
  (params (StateIndex :type Integer))
  (if (`self.IsRewindEnabled`)
    (set `self.IsActiveMontageHandled` false)
    (`BlueprintMapLibrary.Map_Add` (`self.RewindStates`) StateIndex (make `/Game/Blueprints/RewindManager/RewindState` (`SceneComponent.K2_GetComponentToWorld` (`self.RewindableComponent`)) (make `/Game/Blueprints/RewindManager/RewindMontageState` (`self.RewindableSkeletalMesh`) (`self.RewindableActiveMontage`) (`self.RewindableActiveBackwardMontage`) (`self.RewindableBackwardMontage`) (`self.RewindableSlowMontage`) (`self.RewindableBackwardMontagePosition`)) (`self.RewindableMaterialState`) (`self.RewindableCollisionResponseToChannelState`) (`self.RewindableIntegers`) (`self.RewindableIsDeath`)))
    (set `self.RewindableBackwardMontage` null)
    (set `self.RewindableSlowMontage` null)
    (`BlueprintMapLibrary.Map_Clear` (`self.RewindableIntegers`))
    (set `self.RewindableIsDeath` false)
    (set `self.RewindableMaterialState` (struct))
    (set `self.RewindableCollisionResponseToChannelState` (struct))))

(event `/Game/Blueprints/RewindManager/Rewindable.RemoveRewindState`
  (params (StateIndex :type Integer))
  (`BlueprintMapLibrary.Map_Remove` (`self.RewindStates`) StateIndex))

(event `self.ReceiveBeginPlay`
  (set `self.RewindManager` (`self.GetComponentByClass` (`GameplayStatics.GetGameMode`) "/Game/Blueprints/RewindManager/RewindManager.RewindManager_C")))

(event `ApplyRewindalbeInteger`
  (params (IntegerName :type Name) (Value :type Integer)))

(event `ApplyRewindableIsDeath`
  (params (NotDeath :type Boolean)))

(event `/Game/Blueprints/RewindManager/Rewindable.SetRewindableComponent`
  (params (Component :type "SceneComponent Object Reference"))
  (set `self.RewindableComponent` Component))

(event `/Game/Blueprints/RewindManager/Rewindable.SetRewindableMesh`
  (params (Mesh :type "SkeletalMeshComponent Object Reference"))
  (set `self.RewindableSkeletalMesh` Mesh))

(event `PlayRewindableMontage`
  (params (InSkeletalMeshComponent :type "SkeletalMeshComponent Object Reference") (BaseMontage :type "AnimMontage Object Reference") (BackwardMontage :type "AnimMontage Object Reference") (SlowMontage :type "AnimMontage Object Reference") (PlayRate :type "Float (double-precision)" :default 1.0) (StartingPosition :type "Float (double-precision)") (CallbackEventName :type Name))
  (bind _returnvalue (`SkeletalMeshComponent.GetAnimInstance` InSkeletalMeshComponent))
  (bind _rewindableactivemontage (`self.RewindableActiveMontage`))
  (if (not (`/Game/Blueprints/RewindManager/RewindManager.IsTimeManipulationInProgress` (`self.RewindManager`)))
    (if (`KismetSystemLibrary.IsValid` _rewindableactivemontage)
      (set `self.RewindableBackwardMontagePosition` (- (`AnimSequenceBase.SequenceLength` _rewindableactivemontage) (`AnimInstance.Montage_GetPosition` _returnvalue _rewindableactivemontage)))
      (set `self.RewindableBackwardMontage` (`self.RewindableActiveBackwardMontage`))
      (set `self.RewindableActiveMontage` null)
      (set `self.RewindableActiveBackwardMontage` null)
      (`self.OnCompleteRewindableMontage` (`self.LastInvokedRewindableMontageName`)))
    (set `self.RewindableActiveMontage` BaseMontage)
    (set `self.RewindableActiveBackwardMontage` BackwardMontage)
    (set `self.RewindableSlowMontage` SlowMontage)
    (set `self.LastInvokedRewindableMontageName` CallbackEventName)
    (bind _returnvalue_2 (`AnimInstance.Montage_Play` _returnvalue (`self.RewindableActiveMontage`) PlayRate "MontageLength" StartingPosition true))
    (`KismetSystemLibrary.RetriggerableDelay` _returnvalue_2)
    (set `self.RewindableBackwardMontagePosition` 0.0)
    (set `self.RewindableBackwardMontage` BackwardMontage)
    (set `self.RewindableActiveMontage` null)
    (set `self.RewindableActiveBackwardMontage` null)
    (`self.OnCompleteRewindableMontage` (`self.LastInvokedRewindableMontageName`))))

(event `OnCompleteRewindableMontage`
  (params (Name :type "Name (by ref)")))

(event `/Game/Blueprints/RewindManager/Rewindable.StopRepeat`
  (bind _rewindableactivemontage (`self.RewindableActiveMontage`))
  (bind _activemontagepositionlastposition (`self.ActiveMontagePositionLastPosition`))
  (bind _returnvalue (`SkeletalMeshComponent.GetAnimInstance` (`self.RewindableSkeletalMesh`)))
  (bind _returnvalue_2 (`AnimInstance.GetCurrentActiveMontage` _returnvalue))
  ;[1 1 1] Handle continue last played montage
  (if (and (`self.ShouldHandleLastPlayedMontage`) (`KismetSystemLibrary.IsValid` _returnvalue_2))
    (`self.StopAnimMontage` _returnvalue_2)
    (`AnimInstance.Montage_Play` _returnvalue _rewindableactivemontage 1.0 "MontageLength" _activemontagepositionlastposition true)
    (`KismetSystemLibrary.Delay` (- (`AnimSequenceBase.SequenceLength` _rewindableactivemontage) _activemontagepositionlastposition))
    (`self.OnCompleteRewindableMontage` (`self.LastInvokedRewindableMontageName`))))

(event `/Game/Blueprints/RewindManager/Rewindable.SetRewindableInteger`
  (params (Name :type Name) (Value :type Integer))
  (`BlueprintMapLibrary.Map_Add` (`self.RewindableIntegers`) Name Value))

(event `/Game/Blueprints/RewindManager/Rewindable.SetRewindableIsDeath`
  (params (IsDeath :type Boolean))
  (set `self.RewindableIsDeath` IsDeath))

(event `SetRewindableMaterial`
  (params (MaterialTarget :type "PrimitiveComponent Object Reference") (ElementIndex :type Integer) (Material :type "MaterialInterface Object Reference"))
  (set `self.RewindableMaterialState` (make `/Game/Blueprints/RewindManager/RewindMaterialState` MaterialTarget ElementIndex Material (`PrimitiveComponent.GetMaterial` MaterialTarget ElementIndex)))
  (`PrimitiveComponent.SetMaterial` MaterialTarget ElementIndex Material))

(event `SetRewindableCollisionResponseToChannel`
  (params (CollisionTarget :type "PrimitiveComponent Object Reference") (Channel :type "ECollisionChannel Enum" :default "ECC_WorldStatic") (NewResponse :type "ECollisionResponse Enum" :default "ECR_Ignore"))
  (set `self.RewindableCollisionResponseToChannelState` (make `/Game/Blueprints/RewindManager/RewindCollisionResponseToChannelState` CollisionTarget Channel NewResponse (`PrimitiveComponent.GetCollisionResponseToChannel` CollisionTarget Channel)))
  (`PrimitiveComponent.SetCollisionResponseToChannel` CollisionTarget Channel NewResponse))

(fn `UserConstructionScript`)