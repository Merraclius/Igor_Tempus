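; RewindManager drives time rewind for registered Rewindable actors, moving them through record, rewind and repeat phases on Tick.
; Recording advances a shared state index and has each actor collect its state, pruning states beyond a maximum window.
; Rewind steps the index back and switches to repeat at the oldest available state.
; Repeat replays forward at one fifth the index step until reaching the rewind start, then restarts recording.
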(event `self.ReceiveTick`
  (params (DeltaSeconds :type "Float (single-precision)"))
  (if (`self.IsRepeatInProgress`)
    (bind _output_get (set `self.CurrentStateIndex` (+ (`self.CurrentStateIndex`) (/ (`self.StateIndexMultiplier`) 5))))
    (`self.ApplyState` _output_get)
    (if (== (`self.RewindStateIndex`) (`self.CurrentStateIndex`))
      (`self.StopRepeat`))
    (elif (`self.IsRewindInProgress`)
      (bind _output_get_2 (set `self.CurrentStateIndex` (- (`self.CurrentStateIndex`) (`self.StateIndexMultiplier`))))
      (if (or (<= _output_get_2 (`self.StateIndexMultiplier`)) (<= _output_get_2 (`self.LastAvailableRecordStateIndex`)))
        (`self.StartRepeat`)
        (else
          (`self.ApplyState` (`self.CurrentStateIndex`))))
      (else
        (set `self.IsTimeManipulationInProgress` false)
        (if (`self.IsRecordInProgress`)
          (set `self.CurrentStateIndex` (+ (`self.StateIndexMultiplier`) (`self.CurrentStateIndex`)))
          (`self.RecordState` (`self.CurrentStateIndex`))
          (else
            (`KismetSystemLibrary.PrintString` "Waiting rewind state change" true true (struct :`G` 0.66 :`B` 1.0 :`A` 1.0) 0.0)))))))

(fn `ApplyState`
  (params (StateIndex :type Integer))
  (`KismetSystemLibrary.PrintString` (`KismetStringLibrary.Concat_StrStr` "Apply state " (`KismetStringLibrary.Conv_IntToString` StateIndex)) true false (struct :`G` 0.66 :`B` 1.0 :`A` 1.0) 0.0)
  (for _array_element (`self.Actors`)
    (`/Game/Blueprints/RewindManager/Rewindable.ApplyRewindState` _array_element StateIndex (`self.IsRewindInProgress`))
    (if (not true)
      (return))))

(fn `RecordState`
  (params (StateIndex :type Integer))
  (locals (RewindStates :type "Array of Integer"))
  (bind _returnvalue (- StateIndex (`self.MaxStatesSize`)))
  (`KismetSystemLibrary.PrintString` (`KismetStringLibrary.Concat_StrStr` "Record state " (`KismetStringLibrary.Conv_IntToString` StateIndex)) true false (struct :`G` 0.66 :`B` 1.0 :`A` 1.0) 0.0)
  (for _array_element (`self.Actors`)
    (`/Game/Blueprints/RewindManager/Rewindable.CollectRewindState` _array_element StateIndex)
    (if (> StateIndex (`self.MaxStatesSize`))
      (set `self.LastAvailableRecordStateIndex` (+ _returnvalue (`self.StateIndexMultiplier`)))
      (`/Game/Blueprints/RewindManager/Rewindable.RemoveRewindState` _array_element _returnvalue))))

(fn `RegisterEntity`
  (params (Entity :type "Actor Object Reference"))
  (`KismetSystemLibrary.PrintString` (`KismetStringLibrary.Concat_StrStr` "Register entity " (`KismetSystemLibrary.GetDisplayName` Entity)))
  (bind _asrewindable (cast `/Game/Blueprints/RewindManager/Rewindable` Entity)
    (:`then`
      (`KismetArrayLibrary.Array_Add` (`self.Actors`) _asrewindable))
    (:`CastFailed`
      (`KismetSystemLibrary.PrintString` "Can't register to RM"))))

(fn `StartRecord`
  (`KismetSystemLibrary.PrintString` "Start record")
  (set `self.IsRecordInProgress` true)
  (set `self.CurrentStateIndex` 0)
  (set `self.RewindStateIndex` 0)
  (set `self.LastAvailableRecordStateIndex` 0)
  (for _array_element (`self.Actors`)
    (`/Game/Blueprints/RewindManager/Rewindable.StartRecord` _array_element)))

(fn `StartRepeat`
  (if (and (> (`self.RewindStateIndex`) 0) (`self.IsRewindInProgress`))
    (`KismetSystemLibrary.PrintString` "Start repeat")
    (set `self.IsRepeatInProgress` true)
    (set `self.IsTimeManipulationInProgress` true)
    (`self.StopRewind`)
    (for _array_element (`self.Actors`)
      (`/Game/Blueprints/RewindManager/Rewindable.StartRepeat` _array_element))
    (else
      (`KismetSystemLibrary.PrintString` "Can't start repeat"))))

(fn `StartRewind`
  (if (or (`self.IsRepeatInProgress`) (<= (`self.CurrentStateIndex`) (`self.MinStatesSize`)))
    (`KismetSystemLibrary.PrintString` "Can't start rewind")
    (else
      (`KismetSystemLibrary.PrintString` "Start rewind")
      (`self.StopRecord`)
      (set `self.IsRewindInProgress` true)
      (set `self.IsTimeManipulationInProgress` true)
      (set `self.RewindStateIndex` (`self.CurrentStateIndex`))
      (for _array_element (`self.Actors`)
        (`/Game/Blueprints/RewindManager/Rewindable.StartRewind` _array_element)))))

(fn `StopRecord`
  (if (`self.IsRecordInProgress`)
    (`KismetSystemLibrary.PrintString` "Stop record")
    (set `self.IsRecordInProgress` false)
    (else
      (`KismetSystemLibrary.PrintString` "Can't stop record"))))

(fn `StopRepeat`
  (if (`self.IsRepeatInProgress`)
    (`KismetSystemLibrary.PrintString` "Stop repeat")
    (set `self.IsRepeatInProgress` false)
    (for _array_element (`self.Actors`)
      (`/Game/Blueprints/RewindManager/Rewindable.StopRepeat` _array_element))
    (`self.StartRecord`)
    (else
      (`KismetSystemLibrary.PrintString` "Can't stop repeat"))))

(fn `StopRewind`
  (if (`self.IsRewindInProgress`)
    (`KismetSystemLibrary.PrintString` "Stop rewind")
    (set `self.IsRewindInProgress` false)
    (else
      (`KismetSystemLibrary.PrintString` "Can't stop rewind"))))