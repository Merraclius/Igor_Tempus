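; Trigger zone actor that starts and ends linked triggerable actors as something enters or leaves its box in a game with time rewinding.
; Overlaps call TriggerStart or TriggerEnd through TriggerableInterface on every entry in TriggerableActors.
; With TriggeredActors empty, any ThirdPersonCharacter activates it, except a possessed one while the GameMode's RewindManager is manipulating time.
; Otherwise only actors in TriggeredActors activate it, bypassing that time check.
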(event `self.ReceiveBeginPlay`
  (set `self.RewindManager` (`self.GetComponentByClass` (`GameplayStatics.GetGameMode`) "/Game/Blueprints/RewindManager/RewindManager.RewindManager_C")))

(event `self.Box.OnComponentBeginOverlap`
  (params (OverlappedComponent :type "PrimitiveComponent Object Reference") (OtherActor :type "Actor Object Reference") (OtherComp :type "PrimitiveComponent Object Reference") (OtherBodyIndex :type Integer) (bFromSweep :type Boolean) (SweepResult :type "HitResult Structure (by ref)"))
  (bind _istimemanipulationinprogress (`/Game/Blueprints/RewindManager/RewindManager.IsTimeManipulationInProgress` (`self.RewindManager`)))
  (if (<= (`KismetArrayLibrary.Array_Length` (`self.TriggeredActors`)) 0)
    (bind _asthird_person_character (cast `/Game/Blueprints/Character/ThirdPersonCharacter` OtherActor))
    (if (or (not _istimemanipulationinprogress) (and _istimemanipulationinprogress (not (`/Game/Blueprints/Character/MainPlayerCharacter.IsPossesed` _asthird_person_character))))
      (for _array_element (`self.TriggerableActors`) :!label _label
        (bind _astriggerable_interface (cast `/Game/Blueprints/TriggerableInterface` _array_element))
        (`/Game/Blueprints/TriggerableInterface.TriggerStart` _astriggerable_interface)))
    (else
      (for _array_element_2 (`self.TriggeredActors`)
        (if (== _array_element_2 OtherActor)
          (goto _label))))))

(event `self.Box.OnComponentEndOverlap`
  (params (OverlappedComponent :type "PrimitiveComponent Object Reference") (OtherActor :type "Actor Object Reference") (OtherComp :type "PrimitiveComponent Object Reference") (OtherBodyIndex :type Integer))
  (bind _istimemanipulationinprogress (`/Game/Blueprints/RewindManager/RewindManager.IsTimeManipulationInProgress` (`self.RewindManager`)))
  (if (<= (`KismetArrayLibrary.Array_Length` (`self.TriggeredActors`)) 0)
    (bind _asthird_person_character (cast `/Game/Blueprints/Character/ThirdPersonCharacter` OtherActor))
    (if (or (not _istimemanipulationinprogress) (and _istimemanipulationinprogress (not (`/Game/Blueprints/Character/MainPlayerCharacter.IsPossesed` _asthird_person_character))))
      (for _array_element (`self.TriggerableActors`) :!label _label_2
        (bind _astriggerable_interface (cast `/Game/Blueprints/TriggerableInterface` _array_element))
        (`/Game/Blueprints/TriggerableInterface.TriggerEnd` _astriggerable_interface)))
    (else
      (for _array_element_2 (`self.TriggeredActors`)
        (if (== OtherActor _array_element_2)
          (goto _label_2))))))

(fn `UserConstructionScript`)