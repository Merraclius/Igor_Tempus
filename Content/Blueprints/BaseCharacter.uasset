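; Base character Blueprint that manages health, damage and death, with health changes that support time rewind.
; Capsule overlaps with DamagingInterface actors reduce health by their DealDamage value, unless time manipulation is running or ShouldIgnoreDamage returns true.
; ReduceHealth records the prior health as a rewindable integer, which ApplyRewindalbeInteger restores through SetCurrentHealth.
; Death fires only at exactly zero health and calls the empty OnDeath hook; DealDamage is a stub.
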(event `self.ReceiveBeginPlay`
  (`parent.ReceiveBeginPlay`)
  (`self.SetCurrentHealth` (`self.MaxHealth`)))

(event `self.CapsuleComponent.OnComponentBeginOverlap`
  (params (OverlappedComponent :type "PrimitiveComponent Object Reference") (OtherActor :type "Actor Object Reference") (OtherComp :type "PrimitiveComponent Object Reference") (OtherBodyIndex :type Integer) (bFromSweep :type Boolean) (SweepResult :type "HitResult Structure (by ref)"))
  (if (and (not (`/Game/Blueprints/RewindManager/RewindManager.IsTimeManipulationInProgress` (`self.RewindManager`))) (!= OtherActor self))
    (bind _asdamaging_interface (cast `/Game/Blueprints/DamagingInterface` OtherActor))
    (bind _isignored (`/Game/Blueprints/DamagingInterface.ShouldIgnoreDamage`))
    (if (not _isignored)
      (bind _damage (`/Game/Blueprints/DamagingInterface.DealDamage` _asdamaging_interface))
      (`self.ReduceHealth` _damage))))

(event `self.ApplyRewindalbeInteger`
  (params (IntegerName :type Name) (Value :type Integer))
  (switch `name` IntegerName
    (:`CurrentHealth`
      (`self.SetCurrentHealth` Value))))

(event `OnDeath`)

(fn `DealDamage`)

(fn `Death`
  (`self.OnDeath`))

(fn `ReduceHealth`
  (params (Damage :type Integer))
  (returns (Health :type Integer))
  (bind _currenthealth (`self.CurrentHealth`))
  (bind _returnvalue (- _currenthealth Damage))
  (`self.SetRewindableInteger` (`self.RewCurrentHealthName`) _currenthealth)
  (`self.SetCurrentHealth` _returnvalue)
  (return _returnvalue))

(fn `SetCurrentHealth`
  (params (NewHealth :type Integer))
  (bind _output_get (set `self.CurrentHealth` NewHealth))
  (if (== _output_get 0)
    (`self.Death`)))

(fn `ShouldIgnoreDamage`
  (returns (IsIgnored :type Boolean))
  (return false))

(fn `UserConstructionScript`)