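; A rewindable moving door that shuttles its Cube back and forth along a spline.
; On BeginPlay it registers with the game mode's RewindManager, marks the Cube as rewindable and starts the SplineRoute timeline, which positions the Cube and alternates direction on finish.
; Applying rewind state stops the timeline; when collection resumes, a hard-wired branch always restarts it in reverse.
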(event `self.ReceiveBeginPlay`
  (`/Game/Blueprints/RewindManager/RewindManager.RegisterEntity` (`self.GetComponentByClass` (`GameplayStatics.GetGameMode`) "/Game/Blueprints/RewindManager/RewindManager.RewindManager_C") self)
  (`self.SetRewindableComponent` (`self.Cube`))
  (`self.StartMoving`))

(event `self.StartCollectRewindState`
  (if (`self.NeedToStart`)
    (set `self.NeedToStart` false)
    (if true
      (bind (_direction _spline) (`Timeline|SplineRoute` :!via `Reverse` :!label _label)
        (:`Update`
          (`SceneComponent.K2_SetWorldLocation` (`self.Cube`) (`SplineComponent.GetLocationAtTime` (`self.Spline`) _spline "World" false) false false))
        (:`Finished`
          (if (`self.AtTheEnd`)
            (set `self.AtTheEnd` false)
            (goto _label :!via `PlayFromStart`)
            (else
              (set `self.AtTheEnd` true)
              (goto _label :!via `ReverseFromEnd`)))))
      (else
        (goto _label)))))

(event `StartMoving`
  (goto _label))

(event `self.StartApplyRewindState`
  (set `self.NeedToStart` true)
  (goto _label :!via `Stop`))

(fn `UserConstructionScript`)