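; DroppedPlatform is a platform that falls under physics when triggered and works with the time rewind system.
; On BeginPlay it registers with RewindManager, sets its Cube as the rewindable component, and hides its PointLight if inactive, with debug prints.
; TriggerStart, when active, enables physics on the Cube after a delay.
; Tick switches that physics off whenever time manipulation is in progress.
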(event `self.ReceiveBeginPlay`
  (`parent.ReceiveBeginPlay`)
  (`/Game/Blueprints/RewindManager/RewindManager.RegisterEntity` (`self.RewindManager`) self)
  (set `self.RewindableComponent` (`self.Cube`))
  (if (not (`self.IsActive`))
    (`KismetSystemLibrary.PrintString` "Hello")
    (`SceneComponent.SetHiddenInGame` (`self.PointLight`) true false)
    (else
      (`KismetSystemLibrary.PrintString` "no"))))

(event `self.ReceiveTick`
  (params (DeltaSeconds :type "Float (single-precision)"))
  (`parent.ReceiveTick` DeltaSeconds)
  (if (`/Game/Blueprints/RewindManager/RewindManager.IsTimeManipulationInProgress` (`self.RewindManager`))
    (`PrimitiveComponent.SetSimulatePhysics` (`self.Cube`) false)))

(event `/Game/Blueprints/TriggerableInterface.TriggerStart`
  (if (`self.IsActive`)
    (`KismetSystemLibrary.Delay` (`self.TriggerDelay`))
    (`PrimitiveComponent.SetSimulatePhysics` (`self.Cube`) true)))

(fn `UserConstructionScript`
  (`parent.UserConstructionScript`))