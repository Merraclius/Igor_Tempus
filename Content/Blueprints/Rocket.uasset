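; Rocket actor that travels along a spline once triggered and supports the game's rewind system.
; On BeginPlay it registers with the RewindManager and sets its Rocket component as the rewindable component.
; TriggerStart plays the Route timeline, which moves that component to spline locations.
; When rewind state starts applying, a fired rocket stops the timeline and flags it to resume when state collection starts again.
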(event `self.ReceiveBeginPlay`
  (`parent.ReceiveBeginPlay`)
  (`/Game/Blueprints/RewindManager/RewindManager.RegisterEntity` (`self.RewindManager`) self)
  (set `self.RewindableComponent` (`self.Rocket`)))

(event `/Game/Blueprints/TriggerableInterface.TriggerStart`
  (set `self.FireTriggered` true)
  (`self.Fire`))

(event `self.StartCollectRewindState`
  (if (and (`self.FireTriggered`) (`self.NeedToStart`))
    (set `self.NeedToStart` false)
    (bind (_direction _spline) (`Timeline|Route` :!label _label)
      (:`Update`
        (`SceneComponent.K2_SetWorldLocation` (`self.Rocket`) (`SplineComponent.GetLocationAtTime` (`self.Spline`) _spline "World" false) false false)))))

(event `Fire`
  (goto _label))

(event `self.StartApplyRewindState`
  (if (`self.FireTriggered`)
    (set `self.NeedToStart` true)
    (goto _label :!via `Stop`)))

(fn `UserConstructionScript`
  (`parent.UserConstructionScript`))