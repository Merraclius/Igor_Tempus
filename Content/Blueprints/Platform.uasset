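; Moving platform that carries its cube along a spline, looping or one-way with trigger-driven reversal, and supports time rewind.
; Timelines drive the position after an auto or triggered delayed start, recording spline time as rewindable floats and route completion as commands.
; Rewind playback applies those values, though position always uses the loop time, and replays completion commands in the opposite direction.
; StopRewind resumes the active timeline from the restored time.
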(event `self.ReceiveBeginPlay`
  (bind _returnvalue (/ 10.0 (`self.Speed`)))
  (`parent.ReceiveBeginPlay`)
  (`/Game/Blueprints/RewindManager/RewindManager.RegisterEntity` (`self.RewindManager`) self)
  (if (`self.AutoStart`)
    (`self.TriggerStart`)
    (`TimelineComponent.SetPlayRate` (`self.SplineRoute`) _returnvalue)
    (`TimelineComponent.SetPlayRate` (`self.SplineRouteLoop`) _returnvalue)))

(event `self.TriggerStart`
  (`KismetSystemLibrary.Delay` (`self.StartDelay`))
  (`self.PlaySpline`))

(event `PlaySpline`
  (set `self.IsFinished` false)
  (if (`self.IsLoop`)
    (bind (_direction _spline) (`Timeline|SplineRouteLoop`)
      (:`Update`
        (`self.UpdateRewindableLocationFromSpline` _spline (`self.SplineLoopName`))))
    (else
      (bind (_direction_2 _spline_2) (`Timeline|SplineRoute` :!label _label)
        (:`Update`
          (`self.UpdateRewindableLocationFromSpline` _spline_2 (`self.SplineName`)))
        (:`Finished`
          (if (`self.IsReversed`)
            (`self.SetRewindableCommand` (`self.SplineReverseFinishedCommand`))
            (else
              (`self.SetRewindableCommand` (`self.SplineFinishedCommand`))))
          (set `self.IsFinished` true))))))

(event `self.ApplyRewindableCommand`
  (params (Command :type Name))
  (switch `name` Command
    (:`SplineFinished`
      (goto _label :!via `ReverseFromEnd`))
    (:`SplineReverseFinished`
      (goto _label :!via `PlayFromStart`))))

(event `self.TriggerEnd`
  (if (and (`self.IsTriggerEndEnabled`) (not (`self.IsLoop`)))
    (set `self.IsReversed` true)
    (if (`self.IsFinished`)
      (goto _label :!via `ReverseFromEnd`)
      (else
        (goto _label :!via `Reverse`)))))

(event `self.ApplyRewindableFloat`
  (params (Name :type Name) (Value :type "Float (single-precision)"))
  (switch `name` Name
    (:`Spline`
      (set `self.LastRewindableSplineTime` Value))
    (:`SplineLoop`
      (bind _output_get (set `self.LastRewindableSplineLoopTime` Value))))
  (`self.UpdateLocationFromSpline` _output_get)
  (set `self.IsUpdateLocationFromRewFloat` true))

(event `self.StopRewind`
  (bind _splineroute (`self.SplineRoute`))
  (bind _splinerouteloop (`self.SplineRouteLoop`))
  (if (`self.IsUpdateLocationFromRewFloat`)
    (set `self.IsUpdateLocationFromRewFloat` false)
    (if (`self.IsLoop`)
      (`TimelineComponent.SetNewTime` (`self.SplineRouteLoop`) (* 5 (`self.LastRewindableSplineLoopTime`)))
      (if (`TimelineComponent.IsReversing` _splinerouteloop)
        (`TimelineComponent.Reverse` _splinerouteloop)
        (else
          (`TimelineComponent.Play` _splinerouteloop)))
      (else
        (`TimelineComponent.SetNewTime` (`self.SplineRoute`) (* 5 (`self.LastRewindableSplineTime`)))
        (if (`TimelineComponent.IsReversing` _splineroute)
          (`TimelineComponent.Reverse` _splineroute)
          (else
            (`TimelineComponent.Play` _splineroute)))))))

(fn `UpdateLocationFromSpline`
  (params (Time :type "Float (double-precision)"))
  (`SceneComponent.K2_SetWorldLocation` (`self.Cube`) (`SplineComponent.GetLocationAtTime` (`self.Spline`) Time "World" false) false false)
  (return))

(fn `UpdateRewindableLocationFromSpline`
  (params (Time :type "Float (double-precision)") (SplineName :type Name))
  (`self.SetRewindableFloat` SplineName Time)
  (`self.UpdateLocationFromSpline` Time)
  (return))

(fn `UserConstructionScript`)