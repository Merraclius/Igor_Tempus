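; FollowedText is a world text actor that, while triggered, floats above the player and turns its yaw to face the camera.
; TriggerStart and TriggerEnd show or hide it and toggle following through Activate and Deactivate.
; While following, Tick repositions it over the pawn and can swap the original text for alternate strings during RewindManager rewind or repeat, with rewind taking priority.
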(event `self.ReceiveBeginPlay`
  (`parent.ReceiveBeginPlay`)
  (set `self.OriginText` (`TextRenderComponent.Text` (`self.TextRender`))))

(event `/Game/Blueprints/TriggerableInterface.TriggerStart`
  (`self.Activate`))

(event `/Game/Blueprints/TriggerableInterface.TriggerEnd`
  (`self.Deactivate`))

(event `self.ReceiveTick`
  (params (DeltaSeconds :type "Float (single-precision)"))
  (bind _textrender (`self.TextRender`))
  (`parent.ReceiveTick` DeltaSeconds)
  (if (`self.IsFollowed`)
    (if (and (`self.IsShowAltOnRewind`) (`/Game/Blueprints/RewindManager/RewindManager.IsRewindInProgress` (`self.RewindManager`)))
      (`TextRenderComponent.K2_SetText` (`self.TextRender`) (`self.AltTextOnRewind`))
      (elif (and (`self.IsShowAltOnRepeat`) (`/Game/Blueprints/RewindManager/RewindManager.IsRepeatInProgress` (`self.RewindManager`)))
        (`TextRenderComponent.K2_SetText` (`self.TextRender`) (`self.AltTextOnRepeat`))
        (else
          (`TextRenderComponent.K2_SetText` (`self.TextRender`) (`self.OriginText`)))))
    (`SceneComponent.K2_SetWorldLocation` (`self.TextRender`) (`KismetMathLibrary.MakeVector` (.x (`self.K2_GetActorLocation` (`GameplayStatics.GetPlayerPawn` 0))) (.y (`self.K2_GetActorLocation` (`GameplayStatics.GetPlayerPawn` 0))) (+ (.z (`self.K2_GetActorLocation` (`GameplayStatics.GetPlayerPawn` 0))) 100.0)) false false)
    (`SceneComponent.K2_SetWorldRotation` _textrender (`KismetMathLibrary.MakeRotator` (.roll (`SceneComponent.K2_GetComponentRotation` _textrender)) (.pitch (`SceneComponent.K2_GetComponentRotation` _textrender)) (- (.yaw (`self.K2_GetActorRotation` (`GameplayStatics.GetPlayerCameraManager` 0))) 180.0)) false false)))

(fn `Activate`
  (`self.ShowInGame`)
  (set `self.IsFollowed` true))

(fn `Deactivate`
  (`self.HideInGame`)
  (set `self.IsFollowed` false))

(fn `UserConstructionScript`
  (`parent.UserConstructionScript`))