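; Unarmed simple enemy character that takes part in the game's time-rewind system and deals a fixed amount of damage.
; On BeginPlay it registers with the RewindManager, setting its capsule and mesh as rewindable.
; Attack plays a rewindable montage with base, backward and slow variants, guarded against re-entry by an in-progress flag.
; That flag is mirrored to the AI controller and cleared when the montage's named completion callback fires.
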(event `self.ReceiveBeginPlay`
  (`parent.ReceiveBeginPlay`)
  (`/Game/Blueprints/RewindManager/RewindManager.RegisterEntity` (`self.RewindManager`) self)
  (`self.SetRewindableComponent` (`self.CapsuleComponent`))
  (`self.SetRewindableMesh` (`self.Mesh`)))

(event `self.Attack`
  (bind _mainaicontroller (`self.MainAIController`))
  (if (not (`self.IsAttackInProgress`))
    (bind _output_get (set `self.IsAttackInProgress` true))
    (if (`KismetSystemLibrary.IsValid` _mainaicontroller)
      (`/Game/Blueprints/Enemies/MainAiController.UpdateIsAttackInProgress` _mainaicontroller _output_get))
    (`self.PlayRewindableMontage` (`self.Mesh`) "/Game/Animations/Enemy/EnemyAttack/AttackBaseMontage.AttackBaseMontage" "/Game/Animations/Enemy/EnemyAttack/AttackBackwardMontage.AttackBackwardMontage" "/Game/Animations/Enemy/EnemyAttack/AttackSlowMontage.AttackSlowMontage" 1.0 0.0 (`self.MainAttackEventName`))))

(event `self.OnCompleteRewindableMontage`
  (params (Name :type "Name (by ref)"))
  (bind _mainaicontroller (`self.MainAIController`))
  (`parent.OnCompleteRewindableMontage` Name)
  (if (== Name (`self.MainAttackEventName`))
    (bind _output_get (set `self.IsAttackInProgress` false))
    (if (`KismetSystemLibrary.IsValid` _mainaicontroller)
      (`/Game/Blueprints/Enemies/MainAiController.UpdateIsAttackInProgress` _mainaicontroller _output_get))))

(fn `DealDamage`
  (returns (Damage :type Integer))
  (return 10))

(fn `UserConstructionScript`
  (`parent.UserConstructionScript`))