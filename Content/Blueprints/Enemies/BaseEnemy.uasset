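; Base enemy Blueprint with time-rewind support, driven by a cached MainAIController and showing an on-screen HP debug print each tick.
; Combo events toggle weapon capsule collision, DealDamage returns a fixed value, and Attack and vulnerability-window events are empty stubs.
; Death plays rewindable montages, disables AI and collision, and sets a rewindable death flag, whose apply event can re-enable both and swap the material.
; StopRepeat completes the main attack montage and resets the AI.
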(event `self.ReceiveTick`
  (params (DeltaSeconds :type "Float (single-precision)"))
  (`parent.ReceiveTick` DeltaSeconds)
  (`KismetSystemLibrary.PrintString` (`KismetStringLibrary.Concat_StrStr` "Enemy HP: " (`KismetStringLibrary.Conv_IntToString` (`self.CurrentHealth`)) "/" (`KismetStringLibrary.Conv_IntToString` (`self.AccumulatedDamage`))) true false (struct :`R` 1.0 :`G` 0.01492 :`A` 1.0) 0.0))

(event `self.ReceiveBeginPlay`
  (`parent.ReceiveBeginPlay`)
  (bind _asmain_aicontroller (cast `/Game/Blueprints/Enemies/MainAiController` (`self.GetController`)))
  (set `self.MainAIController` _asmain_aicontroller))

(event `Attack`)

(event `ComboAttackSave`
  (`PrimitiveComponent.SetCollisionEnabled` (`self.WeaponCapsule`) "QueryOnly"))

(event `ResetCombo`
  (`PrimitiveComponent.SetCollisionEnabled` (`self.WeaponCapsule`) "NoCollision"))

(event `self.OnDeath`
  (bind _returnvalue (`AnimInstance.GetCurrentActiveMontage` (`SkeletalMeshComponent.GetAnimInstance` (`self.RewindableSkeletalMesh`))))
  (`parent.OnDeath`)
  (if (`KismetSystemLibrary.IsValid` _returnvalue)
    (`self.StopAnimMontage` _returnvalue))
  (`self.PlayRewindableMontage` (`self.Mesh`) "/Game/Animations/Enemy/Death/DeathForwardMontage.DeathForwardMontage" "/Game/Animations/Enemy/Death/DeathBackwardMontage.DeathBackwardMontage" "/Game/Animations/Enemy/Death/DeathSlowMontage.DeathSlowMontage" 1.0 0.0 (`self.DeathMontageEventName`))
  (`self.SetRewindableIsDeath` true)
  (`/Game/Blueprints/Enemies/MainAiController.UpdateIsDisabled` (`self.MainAIController`) true)
  (`PrimitiveComponent.SetCollisionEnabled` (`self.CapsuleComponent`) "NoCollision")
  (`PrimitiveComponent.SetCollisionEnabled` (`self.WeaponCapsule`) "NoCollision"))

(event `self.ApplyRewindableIsDeath`
  (params (NotDeath :type Boolean))
  (`parent.ApplyRewindableIsDeath` NotDeath)
  (if NotDeath
    (`/Game/Blueprints/Enemies/MainAiController.UpdateIsDisabled` (`self.MainAIController`) false)
    (`PrimitiveComponent.SetCollisionResponseToChannel` (`self.CapsuleComponent`) "ECC_GameTraceChannel3" "ECR_Ignore")
    (`self.SetRewindableMaterial` (`self.Mesh`) 0 "/Game/Weapons/InfinityBladeWeapons/Weapons/Dual_Blade/Dual_Blade_WrappedDeath/M_Dual_Blade_WrappedDeath.M_Dual_Blade_WrappedDeath")
    (`PrimitiveComponent.SetCollisionEnabled` (`self.CapsuleComponent`) "QueryAndPhysics")))

(event `OpenVulnerabilityWindow`)

(event `CloseVulnerabilityWindow`)

(event `self.StopRepeat`
  (`parent.StopRepeat`)
  (`self.OnCompleteRewindableMontage` (`self.MainAttackEventName`))
  (`/Game/Blueprints/Enemies/MainAiController.ResetAfterStopRepeat` (`self.MainAIController`)))

(fn `DealDamage`
  (returns (Damage :type Integer))
  (return 20))

(fn `UserConstructionScript`)