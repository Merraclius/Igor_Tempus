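; Behaviour tree task that moves the AI-controlled pawn toward the enemy actor stored in the blackboard.
; On execute it reads the Enemy key as an Actor and runs AIMoveTo, using the AttackRange key as the acceptance radius.
; The task finishes with success or failure from the move result, but never calls FinishExecute if the enemy cast fails.
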(event `self.ReceiveExecuteAI`
  (params (OwnerController :type "AIController Object Reference") (ControlledPawn :type "Pawn Object Reference"))
  (bind _returnvalue (`AIBlueprintHelperLibrary.GetBlackboard` OwnerController))
  (bind _asactor (cast `Actor` (`BlackboardComponent.GetValueAsObject` _returnvalue (`.SelectedKeyName` (break `BlackboardKeySelector` (`self.Enemy`))))))
  (`|AIMoveTo` (`Controller.K2_GetPawn` OwnerController) (0.0 0.0 0.0) _asactor (`BlackboardComponent.GetValueAsFloat` _returnvalue (`.SelectedKeyName` (break `BlackboardKeySelector` (`self.AttackRange`))))
    (:`OnSuccess`
      (`self.FinishExecute` true))
    (:`OnFail`
      (`self.FinishExecute` false))))