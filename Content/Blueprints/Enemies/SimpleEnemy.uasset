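; SimpleEnemy is an enemy Blueprint set up to take part in the game's rewind system.
; On BeginPlay it runs the parent logic, registers itself with the RewindManager, then marks its capsule, mesh and a wrapped-death material on the first mesh slot as rewindable.
; It adds no tick, overlap or construction logic of its own.
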(event `self.ReceiveBeginPlay`
  (`parent.ReceiveBeginPlay`)
  (`/Game/Blueprints/RewindManager/RewindManager.RegisterEntity` (`self.RewindManager`) self)
  (`self.SetRewindableComponent` (`self.CapsuleComponent`))
  (`self.SetRewindableMesh` (`self.Mesh`))
  (`self.SetRewindableMaterial` (`self.Mesh`) 0 "/Game/Weapons/InfinityBladeWeapons/Weapons/Dual_Blade/Dual_Blade_WrappedDeath/M_Dual_Blade_WrappedDeath.M_Dual_Blade_WrappedDeath"))

(fn `UserConstructionScript`
  (`parent.UserConstructionScript`))