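; Enemy AI controller that runs the main behavior tree and feeds player detection and attack range state into its blackboard.
; On BeginPlay it caches the RewindManager from the game mode and starts the tree.
; Perception updates are ignored during time manipulation or for non-player actors; sensing the player sets the sight flag and enemy target, never clearing them.
; StartAttacking and StopAttacking toggle the in-attack-range key.
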(event `self.ReceiveBeginPlay`
  (`parent.ReceiveBeginPlay`)
  (set `self.RewindManager` (`self.GetComponentByClass` (`GameplayStatics.GetGameMode`) "/Game/Blueprints/RewindManager/RewindManager.RewindManager_C"))
  (`self.RunBehaviorTree` "/Game/Blueprints/Enemies/MainAIBehaviourTree.MainAIBehaviourTree"))

(event `self.AIPerception.OnTargetPerceptionUpdated`
  (params (Actor :type "Actor Object Reference") (Stimulus :type "AIStimulus Structure"))
  (if (not (or (`/Game/Blueprints/RewindManager/RewindManager.IsTimeManipulationInProgress` (`self.RewindManager`)) (not (`KismetArrayLibrary.Array_Contains` (`Actor.Tags` Actor) "Player"))))
    (set `self.IsEnemyOnSight` Stimulus_bSuccessfullySensed)
    (if (`self.IsEnemyOnSight`)
      (bind _blackboardcomponent (`self.UseBlackboard` "/Game/Blueprints/Enemies/MainAIBlackboard.MainAIBlackboard"))
      (`BlackboardComponent.SetValueAsBool` _blackboardcomponent (`self.IsEnemyOnSightName`) true)
      (`BlackboardComponent.SetValueAsObject` _blackboardcomponent (`self.EnemyName`) Actor))))

(fn `StartAttacking`
  (bind _blackboardcomponent (`self.UseBlackboard` "/Game/Blueprints/Enemies/MainAIBlackboard.MainAIBlackboard"))
  (`BlackboardComponent.SetValueAsBool` _blackboardcomponent (`self.IsEnemyOnAttackRangeName`) true))

(fn `StopAttacking`
  (bind _blackboardcomponent (`self.UseBlackboard` "/Game/Blueprints/Enemies/MainAIBlackboard.MainAIBlackboard"))
  (`BlackboardComponent.SetValueAsBool` _blackboardcomponent (`self.IsEnemyOnAttackRangeName`) false))

(fn `UserConstructionScript`
  (`parent.UserConstructionScript`))