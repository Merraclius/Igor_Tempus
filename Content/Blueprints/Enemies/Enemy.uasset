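; Enemy character that fights through an AI controller and takes part in the game's time-rewind system.
; It registers with the RewindManager and marks its capsule and mesh as rewindable.
; Attacks play rewindable montages with base, backward and slow variants, syncing attack state to the controller until the completion callback.
; An attack sphere reports range to the controller, ignoring overlap starts during time manipulation, and DealDamage returns fixed damage.
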(event `self.ReceiveBeginPlay`
  (`parent.ReceiveBeginPlay`)
  (bind _asmain_aicontroller (cast `/Game/Blueprints/Enemies/MainAiController` (`self.GetController`)))
  (set `self.MainAIController` _asmain_aicontroller)
  (`/Game/Blueprints/RewindManager/RewindManager.RegisterEntity` (`self.RewindManager`) self)
  (`self.SetRewindableComponent` (`self.CapsuleComponent`))
  (`self.SetRewindableMesh` (`self.Mesh`)))

(event `Attack`
  (bind _mainaicontroller (`self.MainAIController`))
  (if (not (`self.IsAttackInProgress`))
    (bind _output_get (set `self.IsAttackInProgress` true))
    (if (`KismetSystemLibrary.IsValid` _mainaicontroller)
      (`/Game/Blueprints/Enemies/MainAiController.UpdateIsAttackInProgress` _mainaicontroller _output_get))
    (`self.PlayRewindableMontage` (`self.Mesh`) "/Game/Animations/Enemy/Attack/AttackBaseMontage.AttackBaseMontage" "/Game/Animations/Enemy/Attack/AttackBackwardMontage.AttackBackwardMontage" "/Game/Animations/Enemy/Attack/AttackSlowMontage.AttackSlowMontage" 1.0 0.0 "MainAttack")))

(event `self.OnCompleteRewindableMontage`
  (params (Name :type "Name (by ref)"))
  (bind _mainaicontroller (`self.MainAIController`))
  (if (== Name "MainAttack")
    (bind _output_get (set `self.IsAttackInProgress` false))
    (if (`KismetSystemLibrary.IsValid` _mainaicontroller)
      (`/Game/Blueprints/Enemies/MainAiController.UpdateIsAttackInProgress` _mainaicontroller _output_get))))

(event `self.AtackSphere.OnComponentBeginOverlap`
  (params (OverlappedComponent :type "PrimitiveComponent Object Reference") (OtherActor :type "Actor Object Reference") (OtherComp :type "PrimitiveComponent Object Reference") (OtherBodyIndex :type Integer) (bFromSweep :type Boolean) (SweepResult :type "HitResult Structure (by ref)"))
  (if (not (`/Game/Blueprints/RewindManager/RewindManager.IsTimeManipulationInProgress` (`self.RewindManager`)))
    (`/Game/Blueprints/Enemies/MainAiController.UpdateIsEnemyOnAttackRange` (`self.MainAIController`) true)))

(event `self.AtackSphere.OnComponentEndOverlap`
  (params (OverlappedComponent :type "PrimitiveComponent Object Reference") (OtherActor :type "Actor Object Reference") (OtherComp :type "PrimitiveComponent Object Reference") (OtherBodyIndex :type Integer))
  (`/Game/Blueprints/Enemies/MainAiController.UpdateIsEnemyOnAttackRange` (`self.MainAIController`) false))

(fn `DealDamage`
  (returns (Damage :type Integer))
  (return 20))

(fn `UserConstructionScript`)