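; Base character for rewindable enemies that records and replays component transforms and montages for time rewind.
; Montage playback stores slow variants at start and backward variants on completion, which CollectRewindState saves with the transform in an index-keyed map, then clears.
; ApplyRewindState restores the transform and handles backward or slow montages by direction.
; Missing indices lerp transforms between keyframes spaced 100 indices apart.
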(event `/Game/Blueprints/RewindManager/Rewindable.ApplyRewindState`
  (params (StateIndex :type Integer) (IsBackward :type Boolean))
  (bind _rewindablecomponent (`self.RewindableComponent`))
  (bind _rewindstates (`self.RewindStates`))
  (bind (_value _returnvalue) (`BlueprintMapLibrary.Map_Find` (`self.RewindStates`) StateIndex))
  (bind _returnvalue_2 (* (/ StateIndex 100) 100))
  (bind (_transform _montagestate) (break `/Game/Blueprints/RewindManager/RewindState` _value))
  (bind _returnvalue_3 (`SkeletalMeshComponent.GetAnimInstance` (break `/Game/Blueprints/RewindManager/RewindMontageState` _montagestate)))
  (bind _returnvalue_4 (`AnimInstance.GetCurrentActiveMontage` _returnvalue_3))
  (if _returnvalue
    (`SceneComponent.K2_SetWorldTransform` _rewindablecomponent _transform false false)
    (if (and (`KismetSystemLibrary.IsValid` (`.BackwardMontage_15_52C2169F4294B3CFA2B3D5B1071283FE` (break `/Game/Blueprints/RewindManager/RewindMontageState` _montagestate))) IsBackward)
      (if (`KismetSystemLibrary.IsValid` _returnvalue_4)
        (bind _ascharacter (cast `Character` (`AnimInstance.GetOwningActor` _returnvalue_3))
          (:`then`
            (`self.StopAnimMontage` _ascharacter _returnvalue_4))
          (:`CastFailed`
            (`KismetSystemLibrary.PrintString` "CAnt cast to character" true true (struct :`G` 1.0 :`B` 0.553815 :`A` 1.0))))
        (else
          (`|PlayMontage` (break `/Game/Blueprints/RewindManager/RewindMontageState` _montagestate) (`.BackwardMontage_15_52C2169F4294B3CFA2B3D5B1071283FE` (break `/Game/Blueprints/RewindManager/RewindMontageState` _montagestate)))))
      (elif (and (`KismetSystemLibrary.IsValid` (`.SlowMontage_16_036E95F24CB735F24B141BB290ABAEF3` (break `/Game/Blueprints/RewindManager/RewindMontageState` _montagestate))) (not IsBackward))
        (`|PlayMontage` (break `/Game/Blueprints/RewindManager/RewindMontageState` _montagestate) (`.SlowMontage_16_036E95F24CB735F24B141BB290ABAEF3` (break `/Game/Blueprints/RewindManager/RewindMontageState` _montagestate)))))
    (else
      (`SceneComponent.K2_SetWorldTransform` _rewindablecomponent (`KismetMathLibrary.TLerp` (`.Transform_2_6075E1B84316F2D437DB0A86274AD0AB` (break `/Game/Blueprints/RewindManager/RewindState` (`BlueprintMapLibrary.Map_Find` _rewindstates _returnvalue_2))) (`.Transform_2_6075E1B84316F2D437DB0A86274AD0AB` (break `/Game/Blueprints/RewindManager/RewindState` (`BlueprintMapLibrary.Map_Find` _rewindstates (+ _returnvalue_2 100)))) (* (`KismetMathLibrary.Conv_IntToDouble` (mod StateIndex 100)) 0.01)) false false))))

(event `/Game/Blueprints/RewindManager/Rewindable.CollectRewindState`
  (params (StateIndex :type Integer))
  (bind _rewindableslowmontage (`self.RewindableSlowMontage`))
  (bind _rewindablebackwardmontage (`self.RewindableBackwardMontage`))
  (`KismetSystemLibrary.PrintString` (`KismetStringLibrary.Concat_StrStr` "Backward:" (`KismetSystemLibrary.GetDisplayName` _rewindablebackwardmontage) "/Slow" (`KismetSystemLibrary.GetDisplayName` _rewindableslowmontage)) true true (struct :`G` 0.66 :`B` 1.0 :`A` 1.0) 0.0)
  (`BlueprintMapLibrary.Map_Add` (`self.RewindStates`) StateIndex (make `/Game/Blueprints/RewindManager/RewindState` (`SceneComponent.K2_GetComponentToWorld` (`self.RewindableComponent`)) (make `/Game/Blueprints/RewindManager/RewindMontageState` (`self.RewindableSkeletalMesh`) _rewindablebackwardmontage _rewindableslowmontage)))
  (set `self.RewindableBackwardMontage` null)
  (set `self.RewindableSlowMontage` null))

(event `/Game/Blueprints/RewindManager/Rewindable.RemoveRewindState`
  (params (StateIndex :type Integer))
  (`BlueprintMapLibrary.Map_Remove` (`self.RewindStates`) StateIndex))

(event `/Game/Blueprints/RewindManager/Rewindable.SetRewindableComponent`
  (params (Component :type "SceneComponent Object Reference"))
  (set `self.RewindableComponent` Component))

(event `/Game/Blueprints/RewindManager/Rewindable.SetRewindableMesh`
  (params (Mesh :type "SkeletalMeshComponent Object Reference"))
  (set `self.RewindableSkeletalMesh` Mesh))

(event `PlayRewindableMontage`
  (params (InSkeletalMeshComponent :type "SkeletalMeshComponent Object Reference") (BaseMontage :type "AnimMontage Object Reference") (BackwardMontage :type "AnimMontage Object Reference") (SlowMontage :type "AnimMontage Object Reference") (PlayRate :type "Float (double-precision)" :default 1.0) (StartingPosition :type "Float (double-precision)") (StartingSection :type Name))
  (set `self.RewindableSlowMontage` SlowMontage)
  (`|PlayMontage` InSkeletalMeshComponent BaseMontage PlayRate StartingPosition StartingSection
    (:`OnCompleted`
      (set `self.RewindableBackwardMontage` BackwardMontage)
      (`self.OnCompleteRewindableMontage`))
    (:`OnBlendOut`
      (`KismetSystemLibrary.PrintString` "Blend put montage" true true (struct :`R` 1.0 :`B` 0.023098 :`A` 1.0)))
    (:`OnInterrupted`
      (`KismetSystemLibrary.PrintString` "Intepurt montage" true true (struct :`R` 1.0 :`G` 0.091393 :`A` 1.0)))))

(event `OnCompleteRewindableMontage`)

(fn `UserConstructionScript`)