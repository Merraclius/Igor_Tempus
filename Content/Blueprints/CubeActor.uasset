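; CubeActor is a rewindable cube that shuttles back and forth along a spline and registers itself with the RewindManager on BeginPlay.
; The Route timeline drives the cube's world position along the spline, flipping the AtTheEnd direction flag at each finish to ping-pong.
; Applying rewind state stops the timeline, and the next state collection resumes it in the direction given by that flag.
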(event `self.ReceiveBeginPlay`
  (`parent.ReceiveBeginPlay`)
  (`/Game/Blueprints/RewindManager/RewindManager.RegisterEntity` (`self.RewindManager`) self)
  (`self.SetRewindableComponent` (`self.CubeActor`)))

(event `self.StartCollectRewindState`
  ;[1 1 1] Moving by the spline route
  (if (`self.NeedToStart`)
    (set `self.NeedToStart` false)
    (if (`self.AtTheEnd`)
      (bind (_direction _time) (`Timeline|Route` :!via `Reverse` :!label _label)
        (:`Update`
          (`SceneComponent.K2_SetWorldLocation` (`self.CubeActor`) (`SplineComponent.GetLocationAtTime` (`self.Spline`) _time "World" false) false false))
        (:`Finished`
          (if (`self.AtTheEnd`)
            (set `self.AtTheEnd` false)
            (goto _label :!via `PlayFromStart`)
            (else
              (set `self.AtTheEnd` true)
              (goto _label :!via `ReverseFromEnd`)))))
      (else
        (goto _label)))))

(event `FollowTheRoute`
  ;[1 1 1] Moving by the spline route
  (goto _label))

(event `self.StartApplyRewindState`
  (params (IsBackward :type Boolean))
  ;[1 1 1] Moving by the spline route
  (set `self.NeedToStart` true)
  (goto _label :!via `Stop`))

(fn `UserConstructionScript`)