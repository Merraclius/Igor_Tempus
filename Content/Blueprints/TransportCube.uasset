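; TransportCube is a physics cube actor that takes part in the game's time rewind system.
; On BeginPlay it registers itself with the RewindManager and assigns its Cube component as the RewindableComponent.
; Every Tick it sets physics simulation on the Cube to the inverse of the manager's IsTimeManipulationInProgress flag, so physics is off during time manipulation.
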(event `self.ReceiveBeginPlay`
  (`parent.ReceiveBeginPlay`)
  (`/Game/Blueprints/RewindManager/RewindManager.RegisterEntity` (`self.RewindManager`) self)
  (set `self.RewindableComponent` (`self.Cube`)))

(event `self.ReceiveTick`
  (params (DeltaSeconds :type "Float (single-precision)"))
  (`parent.ReceiveTick` DeltaSeconds)
  (`PrimitiveComponent.SetSimulatePhysics` (`self.Cube`) (not (`/Game/Blueprints/RewindManager/RewindManager.IsTimeManipulationInProgress` (`self.RewindManager`)))))

(fn `UserConstructionScript`
  (`parent.UserConstructionScript`))