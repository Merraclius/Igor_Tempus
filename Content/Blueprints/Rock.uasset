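; Rock is a rewindable actor that deals a fixed amount of damage.
; On BeginPlay it registers itself with the RewindManager and sets its Sphere as the RewindableComponent, after running the parent logic.
; DealDamage returns a constant damage value, and ShouldIgnoreDamage always returns false, so the rock never ignores damage.
; Overlap and Tick events are disabled.
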(event `self.ReceiveBeginPlay`
  (`parent.ReceiveBeginPlay`)
  (`/Game/Blueprints/RewindManager/RewindManager.RegisterEntity` (`self.RewindManager`) self)
  (set `self.RewindableComponent` (`self.Sphere`)))

(fn `DealDamage`
  (returns (Damage :type Integer))
  (return 25))

(fn `ShouldIgnoreDamage`
  (returns (IsIgnored :type Boolean))
  (return false))

(fn `UserConstructionScript`
  (`parent.UserConstructionScript`))